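; Tank Blueprint that wires up the barrel reference and drives the player's aiming camera.
; On BeginPlay it passes its Barrel component to SetBarrelRefrece.
; The aimAzimuth axis yaws the AzimuthGimbal and aimAttitude pitches the SpringArm, splitting the two rotations across separate components.
; Both local rotations are scaled by world delta time and a fixed speed, keeping the turn rate frame-rate independent.
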(event EventBeginPlay
  (Class|FinalTank|SetBarrelRefrece (Variables|Default|Getbarrel)))

(event Input|AxisEvents|InputAxisaimAzimuth
  (params (AxisValue :type Float%20%28single-precision%29))
  ;[1 1 1] Camera AimAzimuth
  (Transformation|AddLocalRotation (Variables|Default|GetazimuthGimbal) (Math|Rotator|MakeRotator 0.0 0.0 (* AxisValue (Utilities|Time|GetWorldDeltaSeconds) 25.0)) false false))

(event Input|AxisEvents|InputAxisaimAttitude
  (params (AxisValue :type Float%20%28single-precision%29))
  ;[1 1 1] Camera AimAttitude
  (Transformation|AddLocalRotation (Variables|Default|GetSpringArm) (Math|Rotator|MakeRotator 0.0 (* AxisValue (Utilities|Time|GetWorldDeltaSeconds) 25.0) 0.0) false false))

(fn ConstructionScript)